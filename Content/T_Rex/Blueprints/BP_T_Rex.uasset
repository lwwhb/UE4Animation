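; T-Rex Blueprint that triggers the creature's montage animations through its AB_T_Rex_Locomotion anim instance.
; Each Tick runs set nodes for movement, health, hit and action state, then compares MontageAction with LastMontageAction.
; When they differ, it casts the mesh's anim instance and calls the matching bite, stunned, final kill, roar or patrol function.
; MontageAction then resets to null, so it acts as a one-shot request.
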(event `self.ReceiveTick`
  (params (DeltaSeconds :type "Float (single-precision)"))
  (bind _lastmontageaction (`self.LastMontageAction`))
  (bind _montageaction (`self.MontageAction`))
  (set `self.Speed` (`self.Speed`))
  (set `self.Yaw` (`self.Yaw`))
  (set `self.Pitch` (`self.Pitch`))
  (set `self.Health` (`self.Health`))
  (set `self.Hit_Intensity` (`self.Hit_Intensity`))
  (set `self.Hit_Direction` (`self.Hit_Direction`))
  (set `self.Action` (`self.Action`))
  (if (`|EnumInequality` _montageaction _lastmontageaction)
    (set `self.LastMontageAction` _lastmontageaction)
    (bind _output_get (set `self.MontageAction` _montageaction))
    (bind _asab_t_rex_locomotion (cast `/Game/T_Rex/Animations/Anim_Blueprints/AB_T_Rex_Locomotion` (`SkeletalMeshComponent.GetAnimInstance` (`self.Mesh`))))
    (switch `/Game/T_Rex/Blueprints/E_T_Rex_Montage_Action` _output_get
      (:`NewEnumerator1`
        _)
      (:`NewEnumerator0`
        (`/Game/T_Rex/Animations/Anim_Blueprints/AB_T_Rex_Locomotion.Play_MamaCaveBite_Action` _asab_t_rex_locomotion))
      (:`NewEnumerator2`
        (`/Game/T_Rex/Animations/Anim_Blueprints/AB_T_Rex_Locomotion.Play_Stunned_Action` _asab_t_rex_locomotion))
      (:`NewEnumerator3`
        (`/Game/T_Rex/Animations/Anim_Blueprints/AB_T_Rex_Locomotion.Play_FinalKill_Action` _asab_t_rex_locomotion))
      (:`NewEnumerator4`
        (`/Game/T_Rex/Animations/Anim_Blueprints/AB_T_Rex_Locomotion.Play_RoarStepForward_Action` _asab_t_rex_locomotion))
      (:`NewEnumerator5`
        (`/Game/T_Rex/Animations/Anim_Blueprints/AB_T_Rex_Locomotion.Play_Patrol_Action` _asab_t_rex_locomotion)))
    (set `self.MontageAction` "NewEnumerator1")))

(fn `UserConstructionScript`)